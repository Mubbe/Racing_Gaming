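; BP_Car is a car pawn prototype with force-based driving and a networking test.
; Pressing W calls a server-named driving event that prints whether it runs with authority and uses a FlipFlop to toggle IsA.
; While IsA is true, Tick pushes CapsuleCollision along the actor's forward vector with a large constant force.
; MoveForward and MoveRight axes separately feed standard movement input along the forward and right vectors.
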(event `self.ReceiveBeginPlay`)

(event `Server_ApplyDrivingForce`
  (`/Engine/EditorBlueprintResources/ActorMacros.Switch Has Authority`
    (:`Authority`
      (`KismetSystemLibrary.PrintString` "serveer"))
    (:`Remote`
      (`KismetSystemLibrary.PrintString` "Client")))
  (bind _isa (`/Engine/EditorBlueprintResources/StandardMacros.FlipFlop`)
    (:`A`
      _)
    (:`B`
      _))
  (set `self.Is A` _isa))

(event `Key|W`
  (params (Key :type "Key Structure"))
  (:`Pressed`
    (`self.Server_ApplyDrivingForce`)))

(event `self.ReceiveTick`
  (params (DeltaSeconds :type "Float (single-precision)"))
  (if (`self.Is A`)
    (`PrimitiveComponent.AddForce` (`self.CapsuleCollision`) (* (`self.GetActorForwardVector`) 1000000.0) "None" false)))

(event `InputAxis|MoveForward`
  (params (AxisValue :type "Float (single-precision)"))
  (`self.AddMovementInput` (`self.GetActorForwardVector`) AxisValue))

(event `InputAxis|MoveRight`
  (params (AxisValue :type "Float (single-precision)"))
  (`self.AddMovementInput` (`self.GetActorRightVector`) AxisValue))

(fn `UserConstructionScript`)