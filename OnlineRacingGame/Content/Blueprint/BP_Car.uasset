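; BP_Car is a physics-driven racing car with drifting, boosts and lap timing.
; Tick smooths throttle and steering inputs, then applies forward force, speed-scaled turning torque and lateral grip force to the capsule.
; Drifting changes grip and turning, and a long enough drift grants a short acceleration boost, separate from the cooldown-limited ability boost.
; FinishLap tracks the lap count and best time, notifying BP_PlayerController.
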(event `self.ReceiveTick`
  (params (DeltaSeconds :type "Float (single-precision)"))
  (`|ExecutionSequence`
    (:`then_0`
      ; makes the acceleration smooth based on interp speed
      (set `self.CurrentThrottle` (`KismetMathLibrary.FInterpTo` (`self.CurrentThrottle`) (`self.TargetThrottle`) DeltaSeconds 3.0))
      ; Makes steering smooth based on interp speed
      (set `self.CurrentSteering` (`KismetMathLibrary.FInterpTo` (`self.CurrentSteering`) (`self.TargetSteering`) DeltaSeconds 10.0)))
    (:`then_1`
      ; Add the force to the car root based on current throttle
      (`PrimitiveComponent.AddForce` (`self.CapsuleCollision`) (* (`self.GetActorForwardVector`) (* (`KismetMathLibrary.SelectFloat` 2000000.0 1000000.0 (`self.IsDriftBoosting`)) (`self.CurrentThrottle`))) "None" false)
      ; Adds turning force
      ;; The turning power is relative to the speed
      (bind _returnvalue (`PrimitiveComponent.GetPhysicsLinearVelocity` (`self.CapsuleCollision`) "None"))
      (`PrimitiveComponent.AddTorqueInRadians` (`self.CapsuleCollision`) (* (`self.GetActorUpVector`) (* (select `bool` (`self.IsDrifting`) :`false` 1.0 :`true` (`self.DriftTurnMultiplier`)) (* (`self.CurrentSteering`) (`KismetMathLibrary.FInterpEaseInOut` 50000000.0 3000000.0 (`KismetMathLibrary.FClamp` (/ (`KismetMathLibrary.VSize` _returnvalue) 500.0)))))) "None" false))
    (:`then_2`
      ; Applies boost if is boosting was toogled on by the player
      (if (`self.isBoosting`)
        (bind _output_get (set `self.BoostDuration` (- (`self.BoostDuration`) DeltaSeconds)))
        (if (< _output_get 0.0)
          (set `self.isBoosting` false)
          (else
            (`PrimitiveComponent.AddForce` (`self.CapsuleCollision`) (* (`self.GetActorForwardVector`) 10000000.0) "None" false)))))
    (:`then_3`
      ; drift system
      (bind _returnvalue_2 (`PrimitiveComponent.GetPhysicsLinearVelocity` (`self.CapsuleCollision`) "None"))
      (`PrimitiveComponent.AddForce` (`self.CapsuleCollision`) (* (* (`self.GetActorRightVector`) (* (* (`KismetMathLibrary.Dot_VectorVector` _returnvalue_2 (`self.GetActorRightVector`)) -1.0) (select `bool` (`self.IsDrifting`) :`false` (`self.NormalGrip`) :`true` (`self.DriftGrip`)))) (`PrimitiveComponent.GetMass` (`self.CapsuleCollision`))) "None" false))
    (:`then_4`
      (if (> (`self.NrOfLaps`) -1)
        (set `self.LapTime` (+ (`self.LapTime`) DeltaSeconds))))
    (:`then_6`
      ; Drift Boost Charge System
      (if (`self.IsDrifting`)
        (set `self.DriftCharge` (+ (`self.DriftCharge`) DeltaSeconds))))))

(event `Server_ApplyDrivingForce`
  (params (Direction :type "Float (double-precision)"))
  ; Event tick, interpolates the current throttle to this
  (set `self.TargetThrottle` Direction))

(event `Server_ApplySteering`
  (params (Direction :type "Float (double-precision)"))
  (set `self.TargetSteering` Direction))

(event `GenericAbility`
  (params (Hud :type "/Game/UI/WBP_HUD Object Reference"))
  ; Generic ability is now a boost - is boosting applies force in event tick and cooldown resets variables
  (if (`self.canBoost`)
    (set `self.isBoosting` true)
    (set `self.canBoost` false)
    (`self.BoostCooldown`)
    (`/Engine/EditorBlueprintResources/StandardMacros.IsValid` Hud
      (:`Is Valid`
        (`/Game/UI/WBP_HUD.ActivateBoostIcon` Hud)))))

(event `BoostCooldown`
  ; Generic ability is now a boost - is boosting applies force in event tick and cooldown resets variables
  (`KismetSystemLibrary.Delay` 10.0)
  (set `self.canBoost` true)
  (set `self.BoostDuration` 0.3))

(event `StartDrift`
  ; Drift Boost Activation & Duration
  (set `self.IsDrifting` true)
  (set `self.DriftCharge` 0.0))

(event `FinishLap`
  (bind _nroflaps (`self.NrOfLaps`))
  (`/Engine/EditorBlueprintResources/StandardMacros.IncrementInt` _nroflaps
    (:`  `
      (if (== _nroflaps 1)
        (set `self.BestLapTime` (`self.LapTime`))
        (set `self.LapTime` 0.0)
        (bind _asbp_player_controller (cast `/Game/Blueprint/BP_PlayerController` (`self.GetController`) :!label _label))
        (`/Game/Blueprint/BP_PlayerController.UpdateNrOfLaps` _asbp_player_controller)
        (elif (> _nroflaps 1)
          (if (< (`self.LapTime`) (`self.BestLapTime`))
            (set `self.BestLapTime` (`self.LapTime`))
            (set `self.LapTime` 0.0)
            (goto _label)
            (else
              (goto _label))))))))

(event `EndDrift`
  ; Drift Boost Activation & Duration
  (set `self.IsDrifting` false)
  (if (>= (`self.DriftCharge`) 1.0)
    (set `self.DriftBoostDuration` 0.5)
    (set `self.IsDriftBoosting` true)
    (`KismetSystemLibrary.Delay` 0.5)
    (set `self.IsDriftBoosting` false)))

(fn `UserConstructionScript`)