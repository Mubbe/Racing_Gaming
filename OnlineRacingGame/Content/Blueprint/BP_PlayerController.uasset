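; Player controller for a networked driving game that links local input and the HUD to the controlled BP_Car.
; On BeginPlay, the local controller adds the Enhanced Input mapping, caches and possesses the car, and creates WBP_HUD.
; Throttle and steering inputs go to the car's server functions, while Ability1 calls its generic ability with the HUD.
; Tick converts the capsule's physics velocity to KPH for the HUD and writes debug controller text.
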(event `self.ReceiveBeginPlay`
  ; Connect the controlls with the controller
  (if (`self.IsLocalPlayerController`)
    (`EnhancedInputSubsystemInterface.AddMappingContext` (subsystem `EnhancedInputLocalPlayerSubsystem`) "/Game/Input/IMC_Controlls.IMC_Controlls" 0 (struct))
    ; Store a reference to the car
    (bind _asbp_car (cast `/Game/Blueprint/BP_Car` (`self.K2_GetPawn`)))
    (bind _output_get (set `self.Car` _asbp_car))
    (`self.Possess` _output_get)
    ; Store a reference to the HUD
    (bind _returnvalue (`|CreateWidget` "/Game/WBP_HUD.WBP_HUD_C" self))
    (bind _output_get_2 (set `self.Hud` _returnvalue))
    (`UserWidget.AddToViewport` _output_get_2 0)
    (else
      (`KismetSystemLibrary.PrintString` "Hello"))))

(event `EnhancedInput|/Game/Input/IA_Throttle`
  (params (ActionValue :type "Float (double-precision)") (ElapsedSeconds :type "Float (double-precision)") (TriggeredSeconds :type "Float (double-precision)") (InputAction :type "InputAction Object Reference" :default "/Game/Input/IA_Throttle.IA_Throttle"))
  ; Controls
  (:`Triggered`
    (`/Game/Blueprint/BP_Car.Server_ApplyDrivingForce` (`self.Car`) ActionValue :!label _label))
  (:`Ongoing`
    (goto _label))
  (:`Canceled`
    (goto _label))
  (:`Completed`
    (goto _label)))

(event `self.ReceiveTick`
  (params (DeltaSeconds :type "Float (single-precision)"))
  (`|ExecutionSequence`
    (:`then_0`
      ; Debug test
      (bind _hud (`self.Hud`)
        (:`then`
          (`/Game/WBP_HUD.SetTestText` _hud (`KismetTextLibrary.Conv_ObjectToText` (`GameplayStatics.GetPlayerController` 0))))
        (:`else`)))
    (:`then_1`
      ; Calculates the speed in cm/s and turns it to KPH
      (bind _returnvalue (`PrimitiveComponent.GetPhysicsLinearVelocity` (`/Game/Blueprint/BP_Car.CapsuleCollision` (`self.Car`)) "None"))
      (`/Game/WBP_HUD.SetHudSpeed` (`self.Hud`) (* (`KismetMathLibrary.VSize` _returnvalue) 0.036)))))

(event `EnhancedInput|/Game/Input/IA_Steering`
  (params (ActionValue :type "Float (double-precision)") (ElapsedSeconds :type "Float (double-precision)") (TriggeredSeconds :type "Float (double-precision)") (InputAction :type "InputAction Object Reference" :default "/Game/Input/IA_Steering.IA_Steering"))
  ; Controls
  (:`Triggered`
    (`/Game/Blueprint/BP_Car.Server_ApplySteering` (`self.Car`) ActionValue :!label _label_2))
  (:`Ongoing`
    (goto _label_2))
  (:`Canceled`
    (goto _label_2))
  (:`Completed`
    (goto _label_2)))

(event `EnhancedInput|/Game/Input/IA_Ability1`
  (params (ActionValue :type Boolean) (ElapsedSeconds :type "Float (double-precision)") (TriggeredSeconds :type "Float (double-precision)") (InputAction :type "InputAction Object Reference" :default "/Game/Input/IA_Ability1.IA_Ability1"))
  ; Controls
  (:`Triggered`
    (`/Game/Blueprint/BP_Car.GenericAbility` (`self.Car`) (`self.Hud`))))

(fn `UserConstructionScript`)