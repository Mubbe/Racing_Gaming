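; Finish line actor that registers lap completions when a BP_Car overlaps its box.
; Cars not already in TriggeredCars get FinishLap called and are added to that list, blocking repeat triggers.
; A single shared ten-second Delay then clears the whole list, so the cooldown is not per car.
; NrOfFinishes increments on every car overlap, including blocked repeats.
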(event `self.Box.OnComponentBeginOverlap`
  (params (OverlappedComponent :type "PrimitiveComponent Object Reference") (OtherActor :type "Actor Object Reference") (OtherComp :type "PrimitiveComponent Object Reference") (OtherBodyIndex :type Integer) (bFromSweep :type Boolean) (SweepResult :type "HitResult Structure (by ref)"))
  (bind _asbp_car (cast `/Game/Blueprint/BP_Car` OtherActor))
  (if (not (`KismetArrayLibrary.Array_Contains` (`self.TriggeredCars`) _asbp_car))
    (`self.StartCarTimer` _asbp_car)
    (`KismetArrayLibrary.Array_AddUnique` (`self.TriggeredCars`) _asbp_car))
  (`/Engine/EditorBlueprintResources/StandardMacros.IncrementInt` (`self.NrOfFinishes`)))

(event `StartCarTimer`
  (params (Car :type "/Game/Blueprint/BP_Car Object Reference"))
  (`/Game/Blueprint/BP_Car.FinishLap` Car)
  (`KismetSystemLibrary.Delay` 10.0)
  (`KismetArrayLibrary.Array_Clear` (`self.TriggeredCars`)))

(fn `UserConstructionScript`)