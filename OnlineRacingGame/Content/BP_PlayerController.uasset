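; Player controller for a drivable car that sets up local input and the HUD.
; On BeginPlay, the local controller adds the Enhanced Input mapping context, caches the possessed BP_Car and creates WBP_HUD.
; Throttle and steering actions pass their values straight to the car's server functions for driving force and steering.
; Tick writes player controller 0's name to the HUD as debug text.
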(event `self.ReceiveBeginPlay`
  ; Connect the controlls with the controller
  (if (`self.IsLocalPlayerController`)
    (`EnhancedInputSubsystemInterface.AddMappingContext` (subsystem `EnhancedInputLocalPlayerSubsystem`) "/Game/IMC_Controlls.IMC_Controlls" 0 (struct))
    ; Store a reference to the car
    (bind _asbp_car (cast `/Game/BP_Car` (`self.K2_GetPawn`)))
    (set `self.Car` _asbp_car)
    ; Store a reference to the HUD
    (bind _returnvalue (`|CreateWidget` "/Game/WBP_HUD.WBP_HUD_C" self))
    (bind _output_get (set `self.Hud` _returnvalue))
    (`UserWidget.AddToViewport` _output_get 0)))

(event `self.ReceiveTick`
  (params (DeltaSeconds :type "Float (single-precision)"))
  ; Debug test
  (bind _hud (`self.Hud`)
    (:`then`
      (`/Game/WBP_HUD.SetTestText` _hud (`KismetTextLibrary.Conv_ObjectToText` (`GameplayStatics.GetPlayerController` 0))))
    (:`else`)))

(event `EnhancedInput|/Game/IA_Throttle`
  (params (ActionValue :type "Float (double-precision)") (ElapsedSeconds :type "Float (double-precision)") (TriggeredSeconds :type "Float (double-precision)") (InputAction :type "InputAction Object Reference" :default "/Game/IA_Throttle.IA_Throttle"))
  ; Controls
  (:`Triggered`
    (`/Game/BP_Car.Server_ApplyDrivingForce` (`self.Car`) ActionValue)))

(event `EnhancedInput|/Game/IA_Steering`
  (params (ActionValue :type "Float (double-precision)") (ElapsedSeconds :type "Float (double-precision)") (TriggeredSeconds :type "Float (double-precision)") (InputAction :type "InputAction Object Reference" :default "/Game/IA_Steering.IA_Steering"))
  (:`Triggered`
    (`/Game/BP_Car.Server_ApplySteering` (`self.Car`) ActionValue)))

(fn `UserConstructionScript`)